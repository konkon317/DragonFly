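; Test spawner actor that creates a team-assigned CharacterPawn and reports its death.
; Spawn creates the pawn at the spawner's transform when no valid one exists, stores the reference and sets its team; nothing in this Blueprint calls it.
; Tick polls the pawn's Dead flag and calls OnDead on the first change to true, latched by ActorDead, which is never reset here.
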(event `self.ReceiveBeginPlay`)

(event `self.ReceiveTick`
  (params (DeltaSeconds :type "Float (single-precision)"))
  (bind _spawnactor (`self.SpawnActor`))
  (bind _dead (`/Game/MyContents/BluePrints/Pawn/CharacterPawn.Dead` _spawnactor))
  (if (`KismetSystemLibrary.IsValid` _spawnactor)
    (if (and (== (`self.actorDead`) false) (== _dead true))
      (set `self.actorDead` _dead)
      (`self.OnDead`))))

(fn `spawn`
  (bind (_returnvalue_location _returnvalue_rotation _returnvalue_scale) (`KismetMathLibrary.BreakTransform` (`self.GetTransform`)))
  (if (not (`KismetSystemLibrary.IsValid` (`self.SpawnActor`)))
    (bind _returnvalue (`|SpawnActorFromClass` "/Game/MyContents/BluePrints/Pawn/CharacterPawn.CharacterPawn_C" (`KismetMathLibrary.MakeTransform` _returnvalue_location _returnvalue_rotation _returnvalue_scale) "Undefined" "OverrideRootScale"))
    (set `self.SpawnActor` _returnvalue)
    (set `/Game/MyContents/BluePrints/Pawn/CharacterPawn.characterTeam` (`self.teeam`) _returnvalue)))

(fn `UserConstructionScript`)