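; Gun barrel actor that aims at a moving CharacterPawn target and fires bullets from its muzzle.
; Each tick, RotateToTarget solves a quadratic intercept from target velocity, bullet speed and barrel length to lead the shot.
; It limits relative pitch to about 15 degrees and resets rotation without a target.
; The shot event spawns a bullet ignoring itself and its parent, with sound and a timed muzzle flash.
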(event Custom|shot
  (bind _returnvalue (Game|SpawnActorfromClass "/Game/MyContents/BluePrints/gameObject/Bullet.Bullet_C" (Math|Transform|MakeTransform (Transformation|GetWorldLocation (Variables|Default|Getmuzzle)) (Transformation|GetWorldRotation (Variables|Default|GetScene))) "Undefined" 0 0))
  (for _array_element (Variables|Default|Getignore)
    (Default|AddIgnoreList _returnvalue _array_element)
    (Components|Activation|Activate (Variables|Default|GetParticleSystem) true)
    (Audio|PlaySoundatLocation "/Game/MyContents/sound/Sounds/Weapon_AssaultRifle/Mono/AssaultRifle_Cue.AssaultRifle_Cue" (Transformation|GetWorldLocation (Variables|Default|Getmuzzle)) "0, 0, 0" 0.1 1e+02)
    (Variables|Default|SetMazzleFlashTimer 0.5)))

(event Custom|setParent
  (params (actor :type Actor%20Object%20Reference))
  (bind _output_get (Variables|Default|Setparent actor))
  (Utilities|Array|Add (Variables|Default|Getignore) _output_get))

(event EventBeginPlay
  (Utilities|Array|Add (Variables|Default|Getignore) self)
  (Variables|Default|SetbarrelLength (Math|Vector|VectorLength (- (Transformation|GetWorldLocation (Variables|Default|Getmuzzle)) (Transformation|GetWorldLocation (Variables|Default|GetScene))))))

(event EventActorBeginOverlap
  (params (OtherActor :type Actor%20Object%20Reference)))

(event EventTick
  (params (DeltaSeconds :type Float%20%28single-precision%29))
  (CallFunction|RotatetoTarget)
  (bind _output_get (Variables|Default|SetMazzleFlashTimer (- (Variables|Default|GetMazzleFlashTimer) DeltaSeconds)))
  (if (<= _output_get 0.0)
    (Components|Activation|Deactivate (Variables|Default|GetParticleSystem))))

(fn ConstructionScript)

(fn RotatetoTarget
  (bind _returnvalue (Transformation|GetActorLocation))
  (bind _returnvalue_2 (Math|Trig|Sin(Degrees) 15.0))
  (bind _scene (Variables|Default|GetScene))
  (bind _target (Variables|Default|Gettarget))
  (bind _returnvalue_3 (Transformation|GetActorLocation _target))
  (bind _relativerotation (Variables|/Script/Engine.SceneComponent|GetRelativeRotation _scene))
  (bind _returnvalue_4 (- _returnvalue_3 _returnvalue))
  (bind _returnvalue_5 (Math|Vector|GetForwardVector _relativerotation))
  (bind _returnvalue_6 (Math|Vector|MakeVector 0.0 0.0 (.z _returnvalue_5)))
  (bind _returnvalue_7 (Math|Vector|Normalize _returnvalue_6))
  (bind _returnvalue_8 (* _returnvalue_7 _returnvalue_2))
  (if (and (Utilities|IsValid _target) (Variables|Default|GetHaveTarget))
    (LocalVariables|Setd_minas (Variables|Default|GetbarrelLength))
    (bind _ascharacter_pawn (Utilities|Casting|CastToCharacterPawn _target))
    (Utilities|FlowControl|Sequence
      (:then_0
        (bind _output_get (LocalVariables|SetTargetV (* (Variables|/Game/MyContents/BluePrints/Pawn/CharacterPawn.CharacterPawn_C|Getmoved_speed _ascharacter_pawn) 1.0)))
        (LocalVariables|SetA (- (+ (Math|Float|Power (.x _output_get) 2.0) (Math|Float|Power (.y _output_get) 2.0) (Math|Float|Power (.z _output_get) 2.0)) (Math|Float|Power (LocalVariables|GetBs) 2.0))))
      (:then_1
        (LocalVariables|SetB (* (+ (* (.x _returnvalue_4) (.x _output_get)) (* (.y _returnvalue_4) (.y _output_get)) (* (.z _returnvalue_4) (.z _output_get)) (* (LocalVariables|Getd_minas) (LocalVariables|GetBs))) 2.0)))
      (:then_2
        (LocalVariables|SetC (- (+ (Math|Float|Power (.x _returnvalue_4) 2.0) (Math|Float|Power (.y _returnvalue_4) 2.0) (Math|Float|Power (.z _returnvalue_4) 2.0)) (Math|Float|Power (LocalVariables|Getd_minas) 2.0))))
      (:then_3
        (bind _output_get_2 (LocalVariables|SetD (- (Math|Float|Power (LocalVariables|GetB) 2.0) (* (LocalVariables|GetA) (LocalVariables|GetC) 4.0))))
        (if (> _output_get_2 0.0)
          (LocalVariables|SetDsq (Math|Float|Sqrt _output_get_2))
          (bind _output_get_3 (LocalVariables|SetT1 (/ (+ (* (LocalVariables|GetB) -1.0) (LocalVariables|GetDsq)) (* 2 (LocalVariables|GetA)))))
          (bind _output_get_4 (LocalVariables|SetT2 (/ (- (* (LocalVariables|GetB) -1.0) (LocalVariables|GetDsq)) (* 2 (LocalVariables|GetA)))))))
      (:then_4
        (if (> (Math|Float|SelectFloat (LocalVariables|GetT1) (LocalVariables|GetT2) (> (LocalVariables|GetT1) (LocalVariables|GetT2))) 0.0)
          (Transformation|SetWorldRotation _scene (Math|Rotator|MakeRotationfromAxes (Math|Vector|Normalize (- (+ (* (LocalVariables|GetTargetV) (Math|Float|SelectFloat (LocalVariables|GetT1) (LocalVariables|GetT2) (> (LocalVariables|GetT1) (LocalVariables|GetT2)))) _returnvalue_3) _returnvalue)) "0, 0, 0" "0, 0, 0") false false)
          (if (> (Math|Float|Absolute(Float) (Class|KismetMathLibrary|DegAsin (.z _returnvalue_5))) 15.0)
            (Transformation|SetRelativeRotation _scene (Math|Rotator|MakeRotationfromAxes (+ (* (Math|Vector|Normalize (Math|Vector|MakeVector (.x _returnvalue_5) (.y _returnvalue_5) 0.0)) (- 1.0 (Math|Vector|VectorLength _returnvalue_8))) _returnvalue_8) "0, 0, 0" "0, 0, 0") false false))
          (else
            (CallFunction|ResetRotate)))))
    (else
      (CallFunction|ResetRotate))))

(fn ResetRotate
  (Transformation|SetWorldRotation (Variables|Default|GetScene) (Transformation|GetWorldRotation (Variables|Default|GetDefaultSceneRoot)) false false))