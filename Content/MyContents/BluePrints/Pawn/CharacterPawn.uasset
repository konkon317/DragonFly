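; CharacterPawn is a pawn that constantly travels along its forward vector at a stepped speed and steers left or right.
; SpeedUp and SpeedDown move an index within DesireSpeedList, and Tick eases Speed toward that entry before setting FloatingPawnMovement velocity.
; Turn uses axes built from the root component to blend rotation toward a side, scaled by TurnX and delta time.
; TurnX is only read here.
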(event Custom|SpeedDown
  (bind _speedlevel (Variables|Speed|GetSpeedLevel))
  (if (> _speedlevel 0)
    (Math|Integer|DecrementInt _speedlevel)))

(event Custom|SpeedUp
  (bind _speedlevel (Variables|Speed|GetSpeedLevel))
  (if (< _speedlevel (- (Utilities|Array|Length (Variables|Speed|GetDesireSpeedList)) 1))
    (Math|Integer|IncrementInt _speedlevel)))

(event EventBeginPlay)

(event EventActorBeginOverlap
  (params (OtherActor :type Actor%20Object%20Reference)))

(event EventTick
  (params (DeltaSeconds :type Float%20%28single-precision%29))
  (Variables|Speed|SetSpeed (Math|Float|Lerp (Variables|Speed|GetSpeed) (Utilities|Array|Get(acopy) (Variables|Speed|GetDesireSpeedList) (Variables|Speed|GetSpeedLevel)) 0.5))
  (CallFunction|Turn (Variables|Default|GetTurnX) 0.0 DeltaSeconds)
  (Variables|/Script/Engine.MovementComponent|SetVelocity (Variables|Default|GetFloatingPawnMovement) (* (Transformation|GetActorForwardVector) (Variables|Speed|GetSpeed))))

(fn ConstructionScript)

(fn Turn
  (params (X :type Float%20%28single-precision%29) (Y :type Float%20%28single-precision%29) (DeltaTime :type Float%20%28single-precision%29))
  (bind _output_get (LocalVariables|SetX_cache X))
  (LocalVariables|SetDeltaTime_Cache DeltaTime)
  (|SetLocalValue)
  (if (< _output_get 0.0)
    (LocalVariables|Setnew%20Forward (Math|Rotator|Lerp(Rotator) (LocalVariables|GetForward) (LocalVariables|GetLeft) (* (LocalVariables|GetX_cache) (LocalVariables|GetDeltaTime_Cache) -0.5) true))
    (else
      (LocalVariables|Setnew%20Forward (Math|Rotator|Lerp(Rotator) (LocalVariables|GetForward) (LocalVariables|GetRight) (* (LocalVariables|GetX_cache) (LocalVariables|GetDeltaTime_Cache) 0.5) true))))
  (Transformation|SetActorRotation (LocalVariables|Getnew%20Forward)))