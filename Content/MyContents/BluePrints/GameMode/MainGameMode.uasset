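; Main game mode that tracks the match start countdown and the clear condition.
; Tick decrements the countdown and, once it drops below zero, sets GameStarted and fires the OnGameStart dispatcher.
; After the start, each Tick sets GameClear from whether AliveEnemy equals zero.
; The enemy count is only read here, not updated.
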(event `self.ReceiveTick`
  (params (DeltaSeconds :type "Float (single-precision)"))
  (bind _countdown_tostart (`self.CountDown_ToStart`))
  (set `self.CountDown_ToStart` (- _countdown_tostart DeltaSeconds))
  (if (`self.gameStarted`)
    (set `self.GameClear` (== (`self.AliveEnemy`) 0))
    (elif (< _countdown_tostart 0.0)
      (set `self.gameStarted` true)
      (`self.OnGameStart`))))

(fn `UserConstructionScript`)