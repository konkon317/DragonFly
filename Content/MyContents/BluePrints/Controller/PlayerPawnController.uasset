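; Player controller that relays player input to the possessed CharacterPawn.
; It casts and caches the controlled pawn once at BeginPlay, then every Tick copies camera and move X/Y values into the pawn's Turn and Move variables.
; SpeedUp and SpeedDown input actions call the matching functions on the pawn, with no validity check on the cached reference.
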(event `self.ReceiveBeginPlay`
  (set `self.PawnCache` (cast `/Game/MyContents/BluePrints/Pawn/CharacterPawn` (`self.K2_GetPawn`) :!pure true)))

(event `self.ReceiveTick`
  (params (DeltaSeconds :type "Float (single-precision)"))
  (bind _pawncache (`self.PawnCache`))
  (set `/Game/MyContents/BluePrints/Pawn/CharacterPawn.TurnX` (`self.GetInputAxisValue`) _pawncache)
  (set `/Game/MyContents/BluePrints/Pawn/CharacterPawn.TurnY` (`self.GetInputAxisValue`) _pawncache)
  (set `/Game/MyContents/BluePrints/Pawn/CharacterPawn.MoveX` (`self.GetInputAxisValue`) _pawncache)
  (set `/Game/MyContents/BluePrints/Pawn/CharacterPawn.MoveY` (`self.GetInputAxisValue`) _pawncache))

(event `InputAction|SpeedUp`
  (params (Key :type "Key Structure" :default "AnyKey"))
  (:`Pressed`
    (`/Game/MyContents/BluePrints/Pawn/CharacterPawn.SpeedUp` (`self.PawnCache`))))

(event `InputAction|SpeedDown`
  (params (Key :type "Key Structure" :default "AnyKey"))
  (:`Pressed`
    (`/Game/MyContents/BluePrints/Pawn/CharacterPawn.SpeedDown` (`self.PawnCache`))))

(fn `UserConstructionScript`)