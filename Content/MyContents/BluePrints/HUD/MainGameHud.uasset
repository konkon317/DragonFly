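; Main game HUD that draws targeting markers over actors each frame in DrawHUD, using lists from the player's CharacterPawn.
; In-sight actors not yet targeted get translucent white markers, while targeted actors get amber ones.
; The main target gets a red double marker and a health gauge, cropped by HP ratio and turning red when low.
; MarkerSize scales markers by screen resolution and camera distance, with a maximum size cap.
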(event `self.ReceiveDrawHUD`
  (params (SizeX :type Integer) (SizeY :type Integer))
  (bind _returnvalue (`PlayerCameraManager.GetCameraLocation` (`GameplayStatics.GetPlayerCameraManager` 0)))
  (bind (_ascharacter_pawn _bsuccess) (cast `/Game/MyContents/BluePrints/Pawn/CharacterPawn` (`GameplayStatics.GetPlayerPawn` 0) :!pure true))
  (bind _targetactors (`/Game/MyContents/BluePrints/Pawn/CharacterPawn.TargetActors` _ascharacter_pawn))
  (bind _maintarget (`/Game/MyContents/BluePrints/Pawn/CharacterPawn.MainTarget` _ascharacter_pawn))
  (bind _ascharacter_pawn_2 (cast `/Game/MyContents/BluePrints/Pawn/CharacterPawn` _maintarget :!pure true))
  (bind _returnvalue_2 (/ (`/Game/MyContents/BluePrints/Pawn/CharacterPawn.HitPoint` _ascharacter_pawn_2) (`/Game/MyContents/BluePrints/Pawn/CharacterPawn.HitPointMax` _ascharacter_pawn_2)))
  (if _bsuccess
    (for _array_element (`/Game/MyContents/BluePrints/Pawn/CharacterPawn.InsightActors` _ascharacter_pawn)
      (if (not (`KismetArrayLibrary.Array_Contains` _targetactors _array_element))
        (bind _returnvalue_3 (`self.K2_GetActorLocation` _array_element))
        (bind _sizepx (`self.MarkerSize` _returnvalue_3 _returnvalue SizeX SizeY))
        (bind _returnvalue_4 (/ _sizepx 2.0))
        (`self.DrawTexture` "/Game/MyContents/Texture/hud/target_1.target_1" (- (.x (`self.Project` _returnvalue_3)) _returnvalue_4) (- (.y (`self.Project` _returnvalue_3)) _returnvalue_4) _sizepx _sizepx 0.0 0.0 1.0 1.0 (struct :`R` 1.0 :`G` 1.0 :`B` 1.0 :`A` 0.7) "BLEND_Translucent" 1.0 false 0.0 (0.5 0.5))))
    (for _array_element_2 _targetactors
      (bind _returnvalue_5 (`self.K2_GetActorLocation` _array_element_2))
      (bind _sizepx_2 (`self.MarkerSize` _returnvalue_5 _returnvalue SizeX SizeY))
      (bind _returnvalue_6 (/ _sizepx_2 2.0))
      (bind _returnvalue_7 (- (.x (`self.Project` _returnvalue_5)) _returnvalue_6))
      (bind _returnvalue_8 (- (.y (`self.Project` _returnvalue_5)) _returnvalue_6))
      (bind _returnvalue_9 (== _array_element_2 _maintarget))
      (bind _returnvalue_10 (`KismetMathLibrary.SelectColor` (struct :`R` 1.0 :`G` 0.067612 :`A` 1.0) (struct :`R` 1.0 :`G` 0.715381 :`A` 0.75) _returnvalue_9))
      (`self.DrawTexture` "/Game/MyContents/Texture/hud/target_1.target_1" _returnvalue_7 _returnvalue_8 _sizepx_2 _sizepx_2 0.0 0.0 1.0 1.0 _returnvalue_10 "BLEND_Translucent" 1.0 false 0.0 (0.5 0.5))
      (if _returnvalue_9
        (`self.DrawTexture` "/Game/MyContents/Texture/hud/target_2.target_2" _returnvalue_7 _returnvalue_8 _sizepx_2 _sizepx_2 0.0 0.0 1.0 1.0 _returnvalue_10 "BLEND_Translucent" 1.0 false 0.0 (0.5 0.5))
        (bind _returnvalue_11 (+ _returnvalue_7 (/ (* _sizepx_2 (- 1.0 1.5)) 2.0)))
        (bind _returnvalue_12 (* _sizepx_2 1.5))
        (bind _returnvalue_13 (/ _returnvalue_12 6.0))
        (bind _returnvalue_14 (- _returnvalue_8 (+ _returnvalue_13 (/ _returnvalue_13 2.0))))
        (`self.DrawTexture` "/Game/MyContents/Texture/hud/gage_waku.gage_waku" _returnvalue_11 _returnvalue_14 _returnvalue_12 _returnvalue_13 0.0 0.0 1.0 1.0 (struct :`R` 1.0 :`G` 1.0 :`B` 1.0 :`A` 0.5))
        (`self.DrawTexture` "/Game/MyContents/Texture/hud/gage.gage" _returnvalue_11 _returnvalue_14 (* _returnvalue_12 _returnvalue_2) _returnvalue_13 0.0 0.0 _returnvalue_2 1.0 (`KismetMathLibrary.SelectColor` (struct :`R` 0.985 :`A` 0.5) (struct :`G` 1.0 :`B` 0.070734 :`A` 0.5) (< _returnvalue_2 0.2)))))))

(fn `MarkerSize`
  (params (TargetPos :type "Vector Structure") (CameraPos :type "Vector Structure") (sizeX :type Integer) (sizeY :type Integer))
  (returns (SizePx :type "Float (double-precision)"))
  (bind _returnvalue (`KismetMathLibrary.VSize` (- TargetPos CameraPos)))
  (bind _returnvalue_2 (/ (`KismetMathLibrary.Conv_IntToDouble` sizeX) 1920.0))
  (bind _returnvalue_3 (/ (`KismetMathLibrary.Conv_IntToDouble` sizeY) 1020.0))
  (bind _returnvalue_4 (* (* (`self.size`) (`KismetMathLibrary.SelectFloat` _returnvalue_2 _returnvalue_3 (<= _returnvalue_2 _returnvalue_3))) (`KismetMathLibrary.SelectFloat` 1.0 (/ 2000.0 _returnvalue) (>= _returnvalue 2000.0))))
  (return (`KismetMathLibrary.SelectFloat` 400.0 _returnvalue_4 (>= _returnvalue_4 400.0))))

(fn `UserConstructionScript`)