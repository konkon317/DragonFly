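; Projectile bullet actor that damages whatever it hits, spawns a hit effect and destroys itself.
; Each tick it sphere-traces from its previous position, derived from velocity, to its current one instead of relying on overlap events.
; The hit effect receives the struck actor and the impact offset relative to it.
; Actors added through AddIgnoreList are skipped by the trace, and a timer destroys bullets that hit nothing.
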(event `self.ReceiveBeginPlay`
  (`KismetSystemLibrary.K2_SetTimer` null "destroy" 10.0))

(event `self.ReceiveTick`
  (params (DeltaSeconds :type "Float (single-precision)"))
  (bind _returnvalue (`self.K2_GetActorLocation`))
  (bind (_outhit _returnvalue_2) (`KismetSystemLibrary.SphereTraceSingle_NEW` (- _returnvalue (* (`MovementComponent.Velocity` (`self.ProjectileMovement`)) DeltaSeconds)) _returnvalue (`SphereComponent.GetUnscaledSphereRadius` (`self.Sphere1`)) "TraceTypeQuery1" false (`self.hit ignore list`)))
  (if _returnvalue_2
    (bind (_bblockinghit _binitialoverlap _time _location _impactpoint _normal _impactnormal _physmat _hitactor) (`GameplayStatics.BreakHitResult` _outhit))
    (bind _returnvalue_3 (`|SpawnActorFromClass` "/Game/MyContents/BluePrints/gameObject/hitEffect.hitEffect_C" (`KismetMathLibrary.MakeTransform` _impactpoint (`self.K2_GetActorRotation`)) "Undefined" "OverrideRootScale"))
    (set `/Game/MyContents/BluePrints/gameObject/hitEffect.hitActor` _hitactor _returnvalue_3)
    (set `/Game/MyContents/BluePrints/gameObject/hitEffect.relpos` (- _impactpoint (`self.K2_GetActorLocation` _hitactor)) _returnvalue_3)
    (`GameplayStatics.ApplyDamage` _hitactor 100.0)
    (`self.K2_DestroyActor`)))

(fn `add ignoreList`
  (params (`obj ref` :type "Actor Object Reference"))
  (`KismetArrayLibrary.Array_Add` (`self.hit ignore list`) `obj ref`))

(fn `destroy`
  (`self.K2_DestroyActor`))

(fn `UserConstructionScript`)