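; Blueprint function library of small math helpers for vectors and angles.
; Two functions flatten a vector onto the XY plane by zeroing Z; the normalized variant returns a unit vector, or a zero vector when the input points straight up or down.
; An angle helper wraps degrees into the range above -180 up to 180 by repeatedly adding or subtracting full turns, mapping -180 to 180.
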(fn FlattenVectorNormalized
  (params (in :type Vector))
  (bind _returnvalue (Math|Vector|Normalize in))
  (bind (_x _y _z) (Math|Vector|BreakVector _returnvalue))
  ;[1 1 1] 真上　真下のベクトルならゼロベクトル
  (if (== (Math|Float|Absolute(Float) _z) 1.0)
    (return "")
    (else
      (return (Math|Vector|Normalize (Math|Vector|MakeVector _x _y 0.0))))))

(fn FlattenVector
  (params (in :type Vector))
  (bind (_x _y) (Math|Vector|BreakVector in))
  (return (Math|Vector|MakeVector _x _y 0.0)))

(fn FixAngleDegree
  (params (input :type Float%20%28single-precision%29))
  (bind _output_get (LocalVariables|Settemp input))
  (while (> _output_get 1.8e+02)
    (LocalVariables|Settemp (- (LocalVariables|Gettemp) 3.6e+02)))
  (while (< _output_get -1.8e+02)
    (LocalVariables|Settemp (+ (LocalVariables|Gettemp) 3.6e+02)))
  (if (== _output_get -1.8e+02)
    (LocalVariables|Settemp 1.8e+02))
  (return (LocalVariables|Gettemp)))